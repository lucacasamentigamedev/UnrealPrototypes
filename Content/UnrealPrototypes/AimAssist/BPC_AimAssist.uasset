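; Aim assist component that nudges the owning pawn's view toward a target in front of its camera.
; Init supplies the camera and tuning values, and each tick a debug-drawn multi line trace runs along the camera's forward vector.
; The hit actor with the highest dot product above the threshold becomes the target.
; Its direction, converted to camera space, drives controller pitch and yaw input scaled by delta time and rotation speed.
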(event EventBeginPlay
  ;[0.15 0.15 0.15 0] Get component pawn owner
  (bind _aspawn (Utilities|Casting|CastToPawn (Components|GetOwner)))
  (Variables|Default|SetPawnOwner _aspawn))

(event EventTick
  (params (DeltaSeconds :type Float%20%28single-precision%29))
  (bind _returnvalue (Utilities|Time|GetWorldDeltaSeconds))
  (bind _ownercamera (Variables|Default|GetOwnerCamera))
  (bind _rotationspeed (Variables|Default|GetRotationSpeed))
  (bind _returnvalue_2 (Transformation|GetWorldLocation _ownercamera))
  (bind _returnvalue_3 (* _returnvalue _rotationspeed))
  ;[0.15 0.15 0.145 0] Linetrace from camera in forward for certain distance
  (bind _outhits (Collision|MultiLineTraceByChannel _returnvalue_2 (+ _returnvalue_2 (* (Math|Vector|GetForwardVector _ownercamera) (Variables|Default|GetMaxDistance))) "TraceTypeQuery4" false 0 "ForDuration" true "(R=1.000000,G=0.000000,B=0.000000,A=1.000000)" "(R=0.000000,G=1.000000,B=0.000000,A=1.000000)" 0.05))
  ;[0.15 0.15 0.21 0] Reset max dot and get actors hit
  (Variables|Default|SetMaxDot 0.0)
  (bind _output_get (Variables|Default|SetHitActors _outhits))
  (Variables|Default|SetBestActorToAim 0)
  (for _array_element _output_get
    ;[0.15 0.15 0.15 0] Find best actor by make dot product between camera forward and vector from me to enemy. Taking only dot positive. If is better than the previous and is over the threshold, set the new best actor
    (if (and (> (Math|Vector|DotProduct (Math|Vector|GetForwardVector (Variables|Default|GetOwnerCamera)) (Math|Vector|Normalize (- (Transformation|GetActorLocation (.hitactor _array_element)) (Transformation|GetWorldLocation (Variables|Default|GetOwnerCamera))))) (Variables|Default|GetMaxDot)) (> (Math|Vector|DotProduct (Math|Vector|GetForwardVector (Variables|Default|GetOwnerCamera)) (Math|Vector|Normalize (- (Transformation|GetActorLocation (.hitactor _array_element)) (Transformation|GetWorldLocation (Variables|Default|GetOwnerCamera))))) (Variables|Default|GetDotThreshold)))
      (Variables|Default|SetMaxDot (Math|Vector|DotProduct (Math|Vector|GetForwardVector (Variables|Default|GetOwnerCamera)) (Math|Vector|Normalize (- (Transformation|GetActorLocation (.hitactor _array_element)) (Transformation|GetWorldLocation (Variables|Default|GetOwnerCamera))))))
      (Variables|Default|SetBestActorToAim (.hitactor _array_element))))
  (Utilities|IsValid (Variables|Default|GetBestActorToAim)
    (:Is%20Valid
      ;[0.15 0.15 0.15 0] Rotate toward best enemy
      (bind _result (Math|Float|NegateFloat (* (.pitch (Math|Rotator|MakeRotfromX (Math|Transform|InverseTransformDirection (Transformation|GetWorldTransform (Variables|Default|GetOwnerCamera)) (Math|Vector|Normalize (- (Transformation|GetActorLocation (Variables|Default|GetBestActorToAim)) (Transformation|GetWorldLocation (Variables|Default|GetOwnerCamera))))))) _returnvalue_3))
        (:%20%20
          (Pawn|Input|AddControllerPitchInput (Variables|Default|GetPawnOwner) _result)
          (Pawn|Input|AddControllerYawInput (Variables|Default|GetPawnOwner) (* (.yaw (Math|Rotator|MakeRotfromX (Math|Transform|InverseTransformDirection (Transformation|GetWorldTransform (Variables|Default|GetOwnerCamera)) (Math|Vector|Normalize (- (Transformation|GetActorLocation (Variables|Default|GetBestActorToAim)) (Transformation|GetWorldLocation (Variables|Default|GetOwnerCamera))))))) _returnvalue_3)))))))

(fn Init
  (params (Camera :type Camera%20Component%20Object%20Reference) (MaxDistance :type Float%20%28double-precision%29) (DotThreshold :type Float%20%28double-precision%29) (RotationSpeed :type Float%20%28double-precision%29))
  (Variables|Default|SetOwnerCamera Camera)
  (Variables|Default|SetMaxDistance MaxDistance)
  (Variables|Default|SetDotThreshold DotThreshold)
  (Variables|Default|SetRotationSpeed RotationSpeed))