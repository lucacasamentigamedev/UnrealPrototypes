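; Player aircraft for a flight simulator prototype, flown with keys for throttle, roll and pitch.
; Key events set increments that Tick integrates into a clamped throttle, driving the body mesh's physics velocity along its forward vector.
; Roll and pitch deltas are built as quaternions around the actor's own axes and composed with its current rotation.
; A HUD widget created on BeginPlay receives accumulated roll, pitch and current speed each frame.
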(event EventBeginPlay
  (bind _returnvalue (UserInterface|CreateWidget "/Game/UnrealPrototypes/FlightSimulator/WBP_FlightSimulatorHUD.WBP_FlightSimulatorHUD_C"))
  (bind _output_get (Variables|UI|SetWBP_FlightSimulatorHUDRef _returnvalue))
  (UserInterface|Viewport|AddtoViewport _output_get 0))

(event EventTick
  (params (DeltaSeconds :type Float%20%28single-precision%29))
  (bind _returnvalue (Utilities|Time|GetWorldDeltaSeconds))
  (bind _returnvalue_2 (Utilities|Time|GetWorldDeltaSeconds))
  (bind _rotationspeed (Variables|RotGeneral|GetRotationSpeed))
  (bind _rotationspeed_2 (Variables|RotGeneral|GetRotationSpeed))
  (bind _pitchincrement (Variables|RotPitch|GetPitchIncrement))
  (bind _rollincrement (Variables|RotRoll|GetRollIncrement))
  (bind _returnvalue_3 (* _rollincrement _returnvalue_2 _rotationspeed_2))
  (bind _returnvalue_4 (* _pitchincrement _returnvalue _rotationspeed))
  ;[0.15 0.15 0.15 0.5] Rotate & Move
  ;;[0.15 0.15 0.15 0] Accumulate speed
  (bind _output_get (Variables|Speed|SetSpeedScale (Math|Float|Clamp(Float) (+ (Variables|Speed|GetSpeedScale) (* (* (Utilities|Time|GetWorldDeltaSeconds) 0.2) (Variables|Speed|GetSpeedIncrement))))))
  (Variables|Speed|SetCurrentSpeed (* _output_get (Variables|Speed|GetMaxSpeedScale)))
  ;;[0.15 0.15 0.15 0] Move Player
  (Physics|SetPhysicsLinearVelocity (Variables|Default|GetSMBody) (* (Math|Vector|GetForwardVector (Variables|Default|GetSMBody)) (Variables|Speed|GetCurrentSpeed)) false "None")
  ;;[0.15 0.15 0.15 0.5] Calculate pitch and delta pitch quaternion
  (Variables|RotPitch|SetPitchAngle (+ (Variables|RotPitch|GetPitchAngle) _returnvalue_4))
  (Variables|RotPitch|SetDeltaPitchQuaternion (Math|Conversions|ToQuaternion(Rotator) (Math|Vector|RotatorfromAxisandAngle (Transformation|GetActorRightVector) _returnvalue_4)))
  ;;[0.15 0.15 0.15 0.5] Calculate roll and delta roll quaternion
  (Variables|RotRoll|SetRollAngle (+ (Variables|RotRoll|GetRollAngle) _returnvalue_3))
  (Variables|RotRoll|SetDeltaRollQuaternion (Math|Conversions|ToQuaternion(Rotator) (Math|Vector|RotatorfromAxisandAngle (Transformation|GetActorForwardVector) _returnvalue_3)))
  ;;[0.15 0.15 0.15 0] Rotate Player (roll / pitch)
  (Variables|Rotgeneral|SetCurrentQuaternionRotation (Math|Conversions|ToQuaternion(Rotator) (Transformation|GetActorRotation)))
  (Transformation|SetActorRotation (Class|KismetMathLibrary|QuatRotator (* (* (Variables|RotRoll|GetDeltaRollQuaternion) (Variables|RotPitch|GetDeltaPitchQuaternion)) (Variables|Rotgeneral|GetCurrentQuaternionRotation))))
  (Default|UpdateValue (Variables|UI|GetWBP_FlightSimulatorHUDRef) (Variables|RotRoll|GetRollAngle) (Variables|RotPitch|GetPitchAngle) (Variables|Speed|GetCurrentSpeed)))

(event Input|KeyboardEvents|E
  (params (Key :type Key%20Structure :default "None"))
  ;[0.15 0.15 0.15 0.5] Input
  ;;[0.15 0.15 0.15 0] Speed forth and back
  (:Pressed
    (Variables|Speed|SetSpeedIncrement -1.0))
  (:Released
    (Variables|Speed|SetSpeedIncrement 0.0)))

(event Input|KeyboardEvents|D
  (params (Key :type Key%20Structure :default "None"))
  ;[0.15 0.15 0.15 0.5] Input
  ;;[0.15 0.15 0.15 0] Roll up and down
  (:Pressed
    (Variables|RotRoll|SetRollIncrement -1.0))
  (:Released
    (Variables|RotRoll|SetRollIncrement 0.0)))

(event Input|KeyboardEvents|Q
  (params (Key :type Key%20Structure :default "None"))
  ;[0.15 0.15 0.15 0.5] Input
  ;;[0.15 0.15 0.15 0] Speed forth and back
  (:Pressed
    (Variables|Speed|SetSpeedIncrement 1.0))
  (:Released
    (Variables|Speed|SetSpeedIncrement 0.0)))

(event Input|KeyboardEvents|S
  (params (Key :type Key%20Structure :default "None"))
  ;[0.15 0.15 0.15 0.5] Input
  ;;[0.15 0.15 0.15 0] Pitch left and right
  (:Pressed
    (Variables|RotPitch|SetPitchIncrement -1.0))
  (:Released
    (Variables|RotPitch|SetPitchIncrement 0.0)))

(event Input|KeyboardEvents|A
  (params (Key :type Key%20Structure :default "None"))
  ;[0.15 0.15 0.15 0.5] Input
  ;;[0.15 0.15 0.15 0] Roll up and down
  (:Pressed
    (Variables|RotRoll|SetRollIncrement 1.0))
  (:Released
    (Variables|RotRoll|SetRollIncrement 0.0)))

(event Input|KeyboardEvents|W
  (params (Key :type Key%20Structure :default "None"))
  ;[0.15 0.15 0.15 0.5] Input
  ;;[0.15 0.15 0.15 0] Pitch left and right
  (:Pressed
    (Variables|RotPitch|SetPitchIncrement 1.0))
  (:Released
    (Variables|RotPitch|SetPitchIncrement 0.0)))

(fn ConstructionScript)