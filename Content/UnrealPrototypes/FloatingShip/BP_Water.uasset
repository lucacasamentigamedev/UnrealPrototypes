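; BP_Water is a water volume prototype that floats overlapping actors and carries them along a current.
; FloatingBox and MovingBox overlaps maintain two actor lists, which Tick processes each frame.
; Buoyancy applies Archimedes' principle to bounding-box footprint and depth below WaterLevel, pushing the static mesh upward at the actor's location, scaled by delta time.
; The current is a swept world offset along WaterDirection at WaterSpeed, rather than a force.
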(event OnComponentBeginOverlap(FloatingBox)
  (params (OverlappedComponent :type Primitive%20Component%20Object%20Reference) (OtherActor :type Actor%20Object%20Reference) (OtherComp :type Primitive%20Component%20Object%20Reference) (OtherBodyIndex :type Integer) (bFromSweep :type Boolean) (SweepResult :type Hit%20Result%20Structure%20%28by%20ref%29))
  ;[1 0 0.1309 0.2] Collisions - Detect actors to float
  (Utilities|Array|AddUnique (Variables|Default|GetActorsInWaterToFloat) OtherActor))

(event OnComponentEndOverlap(FloatingBox)
  (params (OverlappedComponent :type Primitive%20Component%20Object%20Reference) (OtherActor :type Actor%20Object%20Reference) (OtherComp :type Primitive%20Component%20Object%20Reference) (OtherBodyIndex :type Integer))
  ;[1 0 0.1309 0.2] Collisions - Detect actors to float
  (Utilities|Array|RemoveItem (Variables|Default|GetActorsInWaterToFloat) OtherActor))

(event OnComponentBeginOverlap(MovingBox)
  (params (OverlappedComponent :type Primitive%20Component%20Object%20Reference) (OtherActor :type Actor%20Object%20Reference) (OtherComp :type Primitive%20Component%20Object%20Reference) (OtherBodyIndex :type Integer) (bFromSweep :type Boolean) (SweepResult :type Hit%20Result%20Structure%20%28by%20ref%29))
  ;[1 0 0.1309 0.2] Collisions - Detect actors to move
  (Utilities|Array|AddUnique (Variables|Default|GetActorsInWaterToMove) OtherActor))

(event OnComponentEndOverlap(MovingBox)
  (params (OverlappedComponent :type Primitive%20Component%20Object%20Reference) (OtherActor :type Actor%20Object%20Reference) (OtherComp :type Primitive%20Component%20Object%20Reference) (OtherBodyIndex :type Integer))
  ;[1 0 0.1309 0.2] Collisions - Detect actors to move
  (Utilities|Array|RemoveItem (Variables|Default|GetActorsInWaterToMove) OtherActor))

(event EventBeginPlay
  ;[0.004252 0 1 0.2] BeginPlay - move water level by the value
  (Transformation|SetRelativeLocation (Variables|Default|GetWater) (Math|Vector|MakeVector 0.0 0.0 (Variables|Default|GetWaterLevel)) false false))

(event EventTick
  (params (DeltaSeconds :type Float%20%28single-precision%29))
  ;[0.15 0.1035 0 0.2] Floating & moving
  (Utilities|FlowControl|Sequence
    (:then_0
      (for _array_element (Variables|Default|GetActorsInWaterToFloat)
        (CallFunction|MakeFloating DeltaSeconds _array_element)))
    (:then_1
      (for _array_element_2 (Variables|Default|GetActorsInWaterToMove)
        (CallFunction|MakeMoving DeltaSeconds _array_element_2 (Variables|Default|GetWater%20Speed) (Variables|Default|GetWater%20Direction))))))

(fn ConstructionScript)

(fn MakeFloating
  (params (DeltaTime :type Float%20%28single-precision%29) (Actor :type Actor%20Object%20Reference))
  (bind (_origin _boxextent) (Collision|GetActorBounds Actor false false))
  ;[1 1 1 0] volume immesed. b * a * p
  (bind _output_get (Variables|Default|SetSubVolume (* (* (* (.x _boxextent) (.y _boxextent)) 4.0) (- (Variables|Default|GetWaterLevel) (- (.z _origin) (.z _boxextent))))))
  ;[1 1 1 0] Add force on on up vector
  (if (not (< (* (* _output_get (Variables|Default|GetDensity)) 9.8) 0.1))
    (Class|PrimitiveComponent|AddForceatLocation (Actor|GetComponentbyClass Actor "/Script/Engine.StaticMeshComponent") (* (* (* (* _output_get (Variables|Default|GetDensity)) 9.8) DeltaTime) (Math|Vector|GetUpVector "0, 0, 0")) (Transformation|GetActorLocation Actor) "None")))

(fn MakeMoving
  (params (DeltaTime :type Float%20%28double-precision%29) (Actor :type Actor%20Object%20Reference) (WaterSpeed :type Float%20%28double-precision%29) (WaterDirection :type Vector))
  (Transformation|AddActorWorldOffset Actor (* (* WaterDirection WaterSpeed) DeltaTime) true true))