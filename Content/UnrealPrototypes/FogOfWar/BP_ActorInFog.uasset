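; BP_ActorInFog is a fog of war actor that fades its mesh's visibility based on a count of overlapping fog volumes.
; UpdateFogVolumeAndCheckTransition adds the passed change to an overlap counter and calls FogTransition only when the above-zero state changes.
; FogTransition plays or reverses a timeline that drives the VisibilityIntensity parameter on a dynamic material instance created at BeginPlay.
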(event Custom|FogTransition
  (params (Show :type Boolean))
  ;[0.15 0.15 0.15 0.5] Blend alpha of material
  (if Show
    (bind _alpha (Timeline|Timeline Play)
      (:Update
        (Rendering|Material|SetScalarParameterValue (Variables|Default|GetDynamicMaterialInstance) "VisibilityIntensity" _alpha :!class /Script/Engine.MaterialInstanceDynamic)))
    (else
      (Timeline|Timeline Reverse))))

(event EventBeginPlay
  ;[0.15 0.15 0.15 0.5] Get dynamic material instance of my SM
  (bind _returnvalue (Rendering|Material|CreateDynamicMaterialInstance (Variables|Default|GetSM) 0 0 "None" :!class /Script/Engine.PrimitiveComponent))
  (Variables|Default|SetDynamicMaterialInstance _returnvalue))

(fn ConstructionScript)

(fn UpdateFogVolumeandCheckTransition
  (params (VolumeCount :type Integer))
  ;[0.15 0.15 0.15 0.5] Add 1 overlap
  (bind _output_get (Variables|Default|SetFogOverlapCounter (+ (Variables|Default|GetFogOverlapCounter) VolumeCount)))
  ;[0.15 0.15 0.15 0.5] If the actual state id ifferent from previous go transition
  (if (!= (not (<= _output_get 0)) (Variables|Default|GetShowTransition))
    (CallFunction|FogTransition (not (<= _output_get 0)))
    (Variables|Default|SetShowTransition (not (<= _output_get 0)))))