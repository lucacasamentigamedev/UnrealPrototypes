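; BP_FogOfWarCharacter is a character that reveals and hides fog-of-war actors within its vision.
; A near sphere and a front box form its vision volumes, and each reports overlaps with BP_ActorInFog actors.
; Begin overlap sends +1 and end overlap sends -1 to UpdateFogVolumeAndCheckTransition, so the fog actor can track overlapping vision volumes and handle its own visibility transition.
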(event OnComponentBeginOverlap(VisionNearSphere)
  (params (OverlappedComponent :type Primitive%20Component%20Object%20Reference) (OtherActor :type Actor%20Object%20Reference) (OtherComp :type Primitive%20Component%20Object%20Reference) (OtherBodyIndex :type Integer) (bFromSweep :type Boolean) (SweepResult :type Hit%20Result%20Structure%20%28by%20ref%29))
  ;[0.15 0.15 0.15 0.5] Show actor in fog
  (bind _asbp_actor_in_fog (Utilities|Casting|CastToBP_ActorInFog OtherActor))
  (Default|UpdateFogVolumeandCheckTransition _asbp_actor_in_fog 1))

(event OnComponentEndOverlap(VisionNearSphere)
  (params (OverlappedComponent :type Primitive%20Component%20Object%20Reference) (OtherActor :type Actor%20Object%20Reference) (OtherComp :type Primitive%20Component%20Object%20Reference) (OtherBodyIndex :type Integer))
  ;[0.15 0.15 0.15 0.5] Hide actor in fog
  (bind _asbp_actor_in_fog (Utilities|Casting|CastToBP_ActorInFog OtherActor))
  (Default|UpdateFogVolumeandCheckTransition _asbp_actor_in_fog -1))

(event OnComponentBeginOverlap(VisionFrontBox)
  (params (OverlappedComponent :type Primitive%20Component%20Object%20Reference) (OtherActor :type Actor%20Object%20Reference) (OtherComp :type Primitive%20Component%20Object%20Reference) (OtherBodyIndex :type Integer) (bFromSweep :type Boolean) (SweepResult :type Hit%20Result%20Structure%20%28by%20ref%29))
  ;[0.15 0.15 0.15 0.5] Show actor in fog
  (bind _asbp_actor_in_fog (Utilities|Casting|CastToBP_ActorInFog OtherActor))
  (Default|UpdateFogVolumeandCheckTransition _asbp_actor_in_fog 1))

(event OnComponentEndOverlap(VisionFrontBox)
  (params (OverlappedComponent :type Primitive%20Component%20Object%20Reference) (OtherActor :type Actor%20Object%20Reference) (OtherComp :type Primitive%20Component%20Object%20Reference) (OtherBodyIndex :type Integer))
  ;[0.15 0.15 0.15 0.5] Hide actor in fog
  (bind _asbp_actor_in_fog (Utilities|Casting|CastToBP_ActorInFog OtherActor))
  (Default|UpdateFogVolumeandCheckTransition _asbp_actor_in_fog -1))

(fn ConstructionScript)