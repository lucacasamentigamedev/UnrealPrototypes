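; Player Blueprint for a force pull and push prototype that binds the mouse buttons to a ForcePullPush object.
; Left click calls FindTarget and right click calls PushTarget, both passing range, radius, a trace channel and the first-person camera.
; Tick calls PullTarget every frame with the pull force as speed and delta time, so left click only picks the target.
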(event EventTick
  (params (DeltaSeconds :type Float%20%28single-precision%29))
  ;[0.15 0.15 0.15 0.5] Pull
  (Class|ForcePullPush|PullTarget (Variables|Default|GetForcePullPush) (Variables|Default|GetPullForce) DeltaSeconds))

(event Input|MouseEvents|LeftMouseButton
  (params (Key :type Key%20Structure :default "None"))
  ;[0.15 0.15 0.15 0.5] Pull
  (:Pressed
    (Class|ForcePullPush|FindTarget (Variables|Default|GetForcePullPush) (Variables|Default|GetForceRange) (Variables|Default|GetForceRadius) "TraceTypeQuery3" (Variables|Default|GetFirstPersonCameraComponent))))

(event Input|MouseEvents|RightMouseButton
  (params (Key :type Key%20Structure :default "None"))
  ;[0.15 0.15 0.15 0.5] Push
  (:Pressed
    (Class|ForcePullPush|PushTarget (Variables|Default|GetForcePullPush) (Variables|Default|GetForceRange) (Variables|Default|GetForceRadius) "TraceTypeQuery3" (Variables|Default|GetFirstPersonCameraComponent) (Variables|Default|GetPushForce))))

(fn ConstructionScript)