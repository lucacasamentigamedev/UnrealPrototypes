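; BP_ParryEnemy is an enemy character for a parry prototype that chases the player and attacks when near.
; Pawn sensing triggers an AI move to the player, then plays the attack montage section, holding an attacking flag for its duration.
; Each tick it checks the player state's parrying flag through an interface against the anim Blueprint's parriable flag, marking itself parried and firing a burst effect when both are true.
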(event OnSeePawn(PawnSensing)
  (params (Pawn :type Pawn%20Object%20Reference))
  ;[0.15 0.15 0.15 0.5] Follow player & attack when near
  (if (not (Variables|Default|GetisAttacking?))
    (AI|AIMoveTo self "0, 0, 0" (Game|Player|GetPlayerPawn 0) 7e+01 false
      (:OnSuccess
        (Components|Movement|StopMovementImmediately (Variables|Character|GetCharacterMovement))
        (Variables|Default|SetisAttacking? true)
        (bind _returnvalue (Animation|PlayAnimMontage "/Game/UnrealPrototypes/Parry/Characters/Enemy/Animations/AM_ParryEnemy.AM_ParryEnemy" 1.0 "Attack"))
        (Utilities|FlowControl|Delay _returnvalue)
        (Variables|Default|SetisAttacking? false)))))

(event EventBeginPlay
  (bind _asabp_parry_enemy (Utilities|Casting|CastToABP_ParryEnemy (Components|SkeletalMesh|GetAnimInstance (Variables|Character|GetMesh))))
  (Variables|Default|SetAs%20ABP%20Parry%20Enemy _asabp_parry_enemy))

(event EventTick
  (params (DeltaSeconds :type Float%20%28single-precision%29))
  (bind _as_abp_parry_enemy (Variables|Default|GetAs%20ABP%20Parry%20Enemy))
  (bind _state (Class|IParry|IGetIsParring(Message) (Game|GetPlayerState 0)))
  (if (and _state (Variables|/Game/UnrealPrototypes/Parry/Characters/Enemy/Animations/ABP_ParryEnemy.ABP_ParryEnemy_C|GetisParriable (Variables|Default|GetAs%20ABP%20Parry%20Enemy)))
    (Variables|/Game/UnrealPrototypes/Parry/Characters/Enemy/Animations/ABP_ParryEnemy.ABP_ParryEnemy_C|SetisParried _as_abp_parry_enemy true)
    (Components|Activation|Activate (Variables|Default|GetNS_Burst) false)
    (else
      (Variables|/Game/UnrealPrototypes/Parry/Characters/Enemy/Animations/ABP_ParryEnemy.ABP_ParryEnemy_C|SetisParried _as_abp_parry_enemy false))))

(fn ConstructionScript)